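; BP_Flipper is a left or right flipper, apparently pinball-style, that swings between a rest and a flipped rotation.
; The construction script picks mirrored start and end rotations from FlyperType, sets the rest pose, and mirrors the right-side component with negative X scale.
; Flip and Flop events use MoveComponentTo to rotate the Flipper component to the end or start rotation over FlipTime.
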(event `self.ReceiveBeginPlay`)

(event `Flip`
  (`KismetSystemLibrary.MoveComponentTo` (`self.Flipper`) (0.0 0.0 0.0) (`self.EndRotation`) false false (`self.FlipTime`)))

(event `Flop`
  (`KismetSystemLibrary.MoveComponentTo` (`self.Flipper`) (0.0 0.0 0.0) (`self.StartRotation`) false false (`self.FlipTime`)))

(fn `UserConstructionScript`
  (bind _flipper (`self.Flipper`))
  (set `self.StartRotation` (select `/Game/Blueprints/FlipType` (`self.FlyperType`) :`NewEnumerator0` (struct :`Yaw` 20.0) :`NewEnumerator1` (struct :`Yaw` -20.0) :!type "Rotator Structure"))
  (set `self.EndRotation` (select `/Game/Blueprints/FlipType` (`self.FlyperType`) :`NewEnumerator0` (struct :`Yaw` -20.0) :`NewEnumerator1` (struct :`Yaw` 20.0) :!type "Rotator Structure"))
  (`SceneComponent.K2_SetRelativeRotation` _flipper (`self.StartRotation`) false false)
  (switch `/Game/Blueprints/FlipType` (`self.FlyperType`)
    (:`NewEnumerator1`
      (`SceneComponent.SetRelativeScale3D` _flipper (-1.0 1.0 1.0)))))