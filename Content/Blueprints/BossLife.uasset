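; BossLife is an actor Blueprint that tracks the hit points of a boss in a pinball game.
; Overlaps with a BP_Ball remove one Life, with a one-second CanBeHit cooldown between hits.
; Tick polls Life and, at zero or below, adds a fixed score through Pinball_GameMode.
; Nothing here guards that award or destroys the actor, so it repeats every tick while Life stays depleted.
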(event `self.ReceiveActorBeginOverlap`
  (params (OtherActor :type "Actor Object Reference"))
  (if (`self.CanBeHit`)
    (cast `/Game/Blueprints/BP_Ball` OtherActor)
    (set `self.Life` (- (`self.Life`) 1))
    (set `self.CanBeHit` false)
    (`KismetSystemLibrary.Delay` 1.0)
    (set `self.CanBeHit` true)))

(event `self.ReceiveTick`
  (params (DeltaSeconds :type "Float (single-precision)"))
  (if (<= (`self.Life`) 0)
    (bind _aspinball_game_mode (cast `/Game/Blueprints/Pinball_GameMode` (`GameplayStatics.GetGameMode`)))
    (`/Game/Blueprints/Pinball_GameMode.AddScore` _aspinball_game_mode 5000.0)))

(fn `UserConstructionScript`)