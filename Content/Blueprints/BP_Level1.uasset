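; BP_Level1 is the first pinball level, which removes itself once the game mode Score exceeds ScoreToLevel2.
; Tick checks the score until a latch is set, then the GoOut timeline lowers DefaultSceneRoot1 along Z.
; When the timeline finishes, the actor is destroyed and ShowLevel is called on NextLevel.
; The Ramp and PoweUp loops feeding the extra DestroyActor call are never executed.
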(event Collision|EventActorBeginOverlap
  (params (OtherActor :type Actor%20Object%20Reference)))

(event EventTick
  (params (DeltaSeconds :type Float%20%28single-precision%29))
  (if (not (Variables|Default|GetAlreadyDisapear))
    (bind _aspinball_game_mode (Utilities|Casting|CastToPinball_GameMode (Game|GetGameMode)))
    (Variables|Default|SetAlreadyDisapear (> (Variables|/Game/Blueprints/Pinball_GameMode.Pinball_GameMode_C|GetScore _aspinball_game_mode) (Variables|Default|GetScoreToLevel2)))
    (if (> (Variables|/Game/Blueprints/Pinball_GameMode.Pinball_GameMode_C|GetScore _aspinball_game_mode) (Variables|Default|GetScoreToLevel2))
      (bind _alpha (Timeline|GoOut PlayFromStart)
        (:Update
          (Transformation|SetRelativeLocation (Variables|Default|GetDefaultSceneRoot1) (Math|Vector|Lerp(Vector) "0, 0, 0" "0,0.000000,-300.000000" _alpha) false false))
        (:Finished
          (Actor|DestroyActor)
          (Actor|DestroyActor (stale _array_element))
          (Default|ShowLevel (Variables|Default|GetNextLevel)))))))

(fn ConstructionScript)