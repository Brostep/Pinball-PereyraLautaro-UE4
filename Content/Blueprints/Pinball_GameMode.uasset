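; Pinball game mode that runs the game from main menu through ball play to high score entry.
; Spawns each ball at the plunger and binds its OnDestroyed to respawn while balls remain, otherwise ending the game.
; At game end, shows high score entry if the saved list is short or its lowest score is beaten, otherwise the main menu.
; Also handles multiplied scoring, reset from class defaults, menu widgets and a cached, lazily loaded or created HighScoreSave.
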(event `self.ReceiveBeginPlay`
  (`self.CreateMainMenu`))

(event `SpawnBall`
  (bind _outactors (`GameplayStatics.GetAllActorsOfClass` "/Game/Blueprints/BP_Plunger.BP_Plunger_C"))
  (bind _returnvalue (`|SpawnActorFromClass` "/Game/Blueprints/BP_Ball.BP_Ball_C" (`KismetMathLibrary.MakeTransform` (`/Game/Blueprints/BP_Plunger.GetBallSpawnLocation` (`|GetArrayItem` _outactors)) (struct) (1.0 1.0 1.0)) "Undefined" "OverrideRootScale" null null))
  (add `self.OnDestroyed` _returnvalue (delegate `OnBallDestroyed`)))

(event `OnBallDestroyed` :!signature `self.OnDestroyed`
  (params (DestroyedActor :type "Actor Object Reference"))
  (if (> (`self.BallLeft`) 0)
    (`self.SpawnBall`)
    (`/Engine/EditorBlueprintResources/StandardMacros.DecrementInt` (`self.BallLeft`))
    (else
      (`self.EndGAme`))))

(event `EndGAme`
  (bind _currentsaveobj (`self.GetSaveGameData`))
  (if (<= (`KismetArrayLibrary.Array_Length` (`/Game/Blueprints/HighScoreSave.SaveStrucs` _currentsaveobj)) 3)
    (`self.CreateHighScoreList` :!label _label)
    (else
      (bind _lowestscorestruc (`/Game/Blueprints/HighScoreSave.DetermineLowestScoreValue` _currentsaveobj))
      (if (< (`.Score_7_CDA01AAE4349E842F211C8AEA4E9D665` (break `/Game/Blueprints/HighScoreStruc` _lowestscorestruc)) (`self.Score`))
        (goto _label)
        (else
          (`self.CreateMainMenu`))))))

(event `ResetGame`
  (bind (_score _multiplier _ballleft) (defaults `/Game/Blueprints/Pinball_GameMode` "Pinball_GameMode_C"))
  (bind _asbp_player_controller (cast `/Game/Blueprints/BP_PlayerController` (`GameplayStatics.GetPlayerController` 0) :!pure true))
  (set `self.Score` _score)
  (set `self.Multiplier` _multiplier)
  (set `self.BallLeft` _ballleft)
  (`self.SpawnBall`)
  (`/Game/Blueprints/BP_PlayerController.CreatePlayerHUD` _asbp_player_controller)
  (set `PlayerController.bShowMouseCursor` false _asbp_player_controller))

(event `CreateHighScoreList`
  (bind _asbp_player_controller (cast `/Game/Blueprints/BP_PlayerController` (`GameplayStatics.GetPlayerController` 0) :!pure true))
  (bind _returnvalue (`|CreateWidget` "/Game/Blueprints/HighScoreEntry.HighScoreEntry_C" _asbp_player_controller))
  (`UserWidget.AddToViewport` _returnvalue 0)
  (set `PlayerController.bShowMouseCursor` true _asbp_player_controller))

(event `CreateMainMenu`
  (bind _asbp_player_controller (cast `/Game/Blueprints/BP_PlayerController` (`GameplayStatics.GetPlayerController` 0) :!pure true))
  (`self.GetSaveGameData`)
  (`WidgetLayoutLibrary.RemoveAllWidgets`)
  (bind _returnvalue (`|CreateWidget` "/Game/Blueprints/MainMenu.MainMenu_C" _asbp_player_controller))
  (`UserWidget.AddToViewport` _returnvalue 0)
  (set `PlayerController.bShowMouseCursor` true _asbp_player_controller))

(event `Create How To play`
  (bind _asbp_player_controller (cast `/Game/Blueprints/BP_PlayerController` (`GameplayStatics.GetPlayerController` 0) :!pure true))
  (`WidgetLayoutLibrary.RemoveAllWidgets`)
  (bind _returnvalue (`|CreateWidget` "/Game/Blueprints/HowToPlay.HowToPlay_C" _asbp_player_controller))
  (`UserWidget.AddToViewport` _returnvalue 0)
  (set `PlayerController.bShowMouseCursor` true _asbp_player_controller))

(fn `AddScore`
  (params (PointToAdd :type "Float (double-precision)"))
  (returns (NewScore :type "Float (double-precision)"))
  (bind _output_get (set `self.Score` (+ (* PointToAdd (`self.Multiplier`)) (`self.Score`))))
  (return _output_get))

(fn `GetSaveGameData`
  (returns (CurrentSaveObj :type "/Game/Blueprints/HighScoreSave Object Reference"))
  (bind _currentsaveobj (`self.CurrentSaveObj`)
    (:`then`
      (return _currentsaveobj))
    (:`else`
      (bind _returnvalue (`GameplayStatics.DoesSaveGameExist` (`self.HighScoreSaveName`)))
      (if _returnvalue
        (bind _returnvalue_2 (`GameplayStatics.LoadGameFromSlot` (`self.HighScoreSaveName`)))
        (bind _ashigh_score_save (cast `/Game/Blueprints/HighScoreSave` _returnvalue_2)
          (:`then`
            (`/Game/Blueprints/HighScoreSave.SortSaveData` _ashigh_score_save)
            (bind _output_get (set `self.CurrentSaveObj` _ashigh_score_save))
            (return _output_get))
          (:`CastFailed`
            _))
        (else
          (bind _returnvalue_3 (`GameplayStatics.CreateSaveGameObject` "/Game/Blueprints/HighScoreSave.HighScoreSave_C"))
          (bind _ashigh_score_save_2 (cast `/Game/Blueprints/HighScoreSave` _returnvalue_3)
            (:`then`
              (bind _output_get_2 (set `self.CurrentSaveObj` _ashigh_score_save_2))
              (return _output_get_2))
            (:`CastFailed`
              _))))
      (return null))))

(fn `UserConstructionScript`)